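; BP_Plane is a plane actor assembled from separate BP_PlanePart components, with damaged and intact variants per part.
; GeneratePlanePart loops over part data, adds a component for each entry and picks the damaged or normal static mesh from its IsBreak flag.
; The hit handlers, construction script and custom event are unfinished stubs, and nothing here calls the generation function.
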(event `CustomEvent`
  (params (NewParam :type "Array of String"))
  (for _array_element NewParam
    (switch `string` _array_element)))

(fn `GeneratePlanePart`
  (locals (NewLocalVar :type String))
  (for _array_element _
    (bind (_normalpart _demagedpart _isbreak) (break `/Game/Trail/Blueprints/Plane/PlaneData/S_PlanePart` _array_element))
    (if _isbreak
      (bind _returnvalue (`|AddComponentByClass` "/Game/Trail/Blueprints/Plane/BP_PlanePart.BP_PlanePart_C"))
      (`StaticMeshComponent.SetStaticMesh` _returnvalue _demagedpart)
      (else
        (bind _returnvalue_2 (`|AddComponentByClass` "/Game/Trail/Blueprints/Plane/BP_PlanePart.BP_PlanePart_C"))
        (`StaticMeshComponent.SetStaticMesh` _returnvalue_2 _normalpart)))))

(fn `HandlePartHit`
  (params (PartIndex :type Integer)))

(fn `OnPartHit`
  (params (PartIndex :type Integer))
  (return))

(fn `UserConstructionScript`)