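; Trial game mode that runs a levelled questionnaire, including a plane-check task with a ladder.
; On BeginPlay it creates the question and check-module managers and places the main widget on the character's widget component.
; Fetching a level's question updates the character's background; plane checks also reprocess questions, toggle movement and show the ladder.
; It relays ray-hit actors to tag and image questions, switching widget collision between pass-through and query-only.
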(event `CustomEvent`)

(event `self.ReceiveBeginPlay`
  (`|ExecutionSequence`
    (:`then_0`
      (bind _returnvalue (`|GenericCreateObject` "/Game/Trail/Blueprints/Questions/BP_QuestionManager.BP_QuestionManager_C"))
      (bind _output_get (set `self.BP_QuestionManager` _returnvalue))
      (`/Game/Trail/Blueprints/Questions/BP_QuestionManager.GenerateQuestionnaire` _output_get))
    (:`then_1`
      (bind _returnvalue_2 (`|GenericCreateObject` "/Script/Overhaul.CheckModuleManager"))
      (bind _output_get_2 (set `self.Plane` _returnvalue_2))
      (`CheckModuleManager.ProcessQuestions` _output_get_2 20))
    (:`then_2`
      (bind _returnvalue_3 (`GameplayStatics.GetActorOfClass` "/Game/Trail/Blueprints/GameMode/BP_ThirdPersonCharacter.BP_ThirdPersonCharacter_C"))
      (bind _output_get_3 (set `self.Character` _returnvalue_3))
      (`/Game/Trail/Blueprints/GameMode/BP_ThirdPersonCharacter.BanMove` _output_get_3 false))
    (:`then_3`
      (bind _returnvalue_4 (`|CreateWidget` "/Game/Trail/UI/UMG_Main.UMG_Main_C"))
      (set `self.UMG` _returnvalue_4)
      (bind _widgetcomponent (`/Game/Trail/Blueprints/GameMode/BP_ThirdPersonCharacter.CreateUI` (`self.Character`)))
      (bind _output_get_4 (set `self.Widget Component` _widgetcomponent))
      (`WidgetComponent.SetWidget` _output_get_4 (`self.UMG`)))))

(fn `ClimbLadder`
  (params (IsClimb :type Boolean))
  (returns (IsTop :type Boolean) (IsBottom :type Boolean) (CurrentHight :type "Float (double-precision)"))
  (bind (_istop _isbottom _currenthight) (`/Game/Trail/Blueprints/GameMode/BP_ThirdPersonCharacter.ClimbLadder` (`self.Character`) IsClimb))
  (return _istop _isbottom _currenthight))

(fn `DestoryImageQuestion`
  (`CheckModuleManager.ProcessLineRayResult` (`self.Plane`) (`self.CurrentImageBox`)))

(fn `DisplayFindTag`
  (params (Index :type Integer))
  (`/Game/Trail/UI/UMG_Main.DisplayFindTag` (`self.UMG`) Index)
  (`KismetSystemLibrary.PrintString` "GameMode"))

(fn `DisplayImageUI`
  (params (Index :type Integer) (Actor :type "Actor Object Reference"))
  (set `self.CurrentImageBox` Actor)
  (`/Game/Trail/UI/UMG_Main.DisplayTFQuestion` (`self.UMG`) Index)
  (`self.EnableThroughUI` false))

(fn `DisplayLadder`
  (params (IsVIsible :type Boolean))
  (locals (MaxHeight :type "Float (double-precision)") (EveryHeight :type "Float (double-precision)") (CurrentHeight :type "Float (double-precision)"))
  (`/Game/Trail/Blueprints/GameMode/BP_ThirdPersonCharacter.DisplayLadder` (`self.Character`) IsVIsible))

(fn `EnableThroughUI`
  (params (IsThrough :type Boolean))
  (bind _widget_component (`self.Widget Component`))
  (if IsThrough
    (`PrimitiveComponent.SetCollisionEnabled` _widget_component "NoCollision")
    (else
      (`PrimitiveComponent.SetCollisionEnabled` _widget_component "QueryOnly"))))

(fn `GetBreakQuestion`
  (params (BreakActor :type "Actor Object Reference"))
  (bind _returnvalue (`CheckModuleManager.ProcessLineRayResult` (`self.Plane`) BreakActor))
  (bind _questionindex (break `ReturnResult` _returnvalue))
  (if (not (== _questionindex -1))
    (`KismetSystemLibrary.PrintString` (`KismetStringLibrary.Conv_IntToString` _questionindex))
    (`self.DisplayFindTag` _questionindex)))

(fn `GetQuestionlData`
  (params (LevelIndex :type Integer))
  (returns (CurrentQuestionModule :type "/Game/Trail/Blueprints/Questions/BP_QuestionModule Object Reference"))
  (bind _currentquestionmodule (`/Game/Trail/Blueprints/Questions/BP_Level.CurrentQuestionModule` (`|GetArrayItem` (`/Game/Trail/Blueprints/Questions/BP_QuestionManager.Levels` (`self.BP_QuestionManager`)) LevelIndex)))
  (switch `/Game/Trail/Blueprints/Questions/E_QuestionType` (`/Game/Trail/Blueprints/Questions/BP_QuestionModule.QuestionType` _currentquestionmodule)
    (:`NewEnumerator0`
      _)
    (:`NewEnumerator1`
      _)
    (:`NewEnumerator2`
      _)
    (:`NewEnumerator4`
      (`CheckModuleManager.ProcessQuestions` (`self.Plane`) 20)
      (`self.EnableThroughUI` true)
      (`/Game/Trail/Blueprints/GameMode/BP_ThirdPersonCharacter.BanMove` (`self.Character`) true)
      (`self.DisplayLadder` true)))
  (`/Game/Trail/Blueprints/GameMode/BP_ThirdPersonCharacter.ChangeBackground` (`self.Character`) (`/Game/Trail/Blueprints/Questions/BP_QuestionModule.CharacterLocation` _currentquestionmodule))
  (return _currentquestionmodule))

(fn `UserConstructionScript`)