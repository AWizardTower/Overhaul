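; Question module that steps through a list of questions within a level and tracks the current one.
; NextQuestion advances the clamped index, sets the current question and reports whether the list and the level have ended.
; When the index reaches the list length, it asks the level reference for the next module, yet still reads the array at that index.
; RandomQuestion is an empty stub.
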(fn `Add Question Index`
  (returns (isLastIndex :type Boolean) (isLevelEnd :type Boolean))
  (bind _returnvalue (`KismetArrayLibrary.Array_Length` (`self.Questions`)))
  (bind _returnvalue_2 (== (`self.CurrentIndex`) _returnvalue))
  (set `self.CurrentIndex` (`KismetMathLibrary.Clamp` (+ (`self.CurrentIndex`) 1) 0 _returnvalue))
  (if _returnvalue_2
    (bind _islevelend (`/Game/Trail/Blueprints/Questions/BP_Level.NextModule` (`self.LevelRef`))))
  (return _returnvalue_2 _islevelend))

(fn `NextQuestion`
  (returns (isLastIndex :type Boolean) (isLevelEnd :type Boolean))
  (`|ExecutionSequence`
    (:`then_0`
      (bind (_islastindex _islevelend) (`self.Add Question Index`)))
    (:`then_1`
      (set `self.CurrentQuestion` (`|GetArrayItem` (`self.Questions`) (`self.CurrentIndex`)))
      (return _islastindex _islevelend))))

(fn `RandomQuestion`
  (params (QuestionNum :type Integer)))