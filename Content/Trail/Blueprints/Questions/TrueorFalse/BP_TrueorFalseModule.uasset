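; BP_TrueorFalseModule loads the true-or-false quiz questions from the DT_TrueorFalse data table.
; RandomQuestion walks every row, stores each found struct in STrueorFalses and wraps it in a constructed BP_TrueorFalseQuestion added to Questions.
; CurrentQuestion is set to the first entry on each pass.
; Despite its name, the function does no shuffling and leaves its QuestionNum input unused.
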(fn `RandomQuestion`
  (params (QuestionNum :type Integer))
  (bind _outrownames (`DataTableFunctionLibrary.GetDataTableRowNames` "/Game/Trail/Blueprints/Questions/QuestionsData/DT_TrueorFalse.DT_TrueorFalse"))
  (for _array_element _outrownames
    (`|ExecutionSequence`
      (:`then_0`
        (bind _returnvalue (`|GetDataTableRow` "/Game/Trail/Blueprints/Questions/QuestionsData/DT_TrueorFalse.DT_TrueorFalse" _array_element)
          (:`then`
            (`KismetArrayLibrary.Array_Add` (`self.S_TrueorFalses`) _returnvalue))))
      (:`then_1`
        (bind _returnvalue_2 (`|GenericCreateObject` "/Game/Trail/Blueprints/Questions/TrueorFalse/BP_TrueorFalseQuestion.BP_TrueorFalseQuestion_C"))
        (set `/Game/Trail/Blueprints/Questions/TrueorFalse/BP_TrueorFalseQuestion.S_TrueorFalse` _returnvalue _returnvalue_2)
        (`KismetArrayLibrary.Array_Add` (`self.Questions`) _returnvalue_2))
      (:`then_2`
        (set `self.CurrentQuestion` (`|GetArrayItem` (`self.Questions`)))))))