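; Quiz module for the plane-check questions that holds question data and tracks the module's total score.
; RandomQuestion copies the DT_CheckPlane and DT_TFImage rows into two maps keyed by each row's Index; despite its name, it does no random selection and ignores QuestionNum.
; AddScore accumulates PlaneTotalScore, and GetModuleScore prints that total as a Chinese debug message and returns it.
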(fn `AddScore`
  (params (Score :type Integer))
  (set `self.PlaneTotalScore` (+ (`self.PlaneTotalScore`) Score)))

(fn `GetModuleScore`
  (returns (Score :type Integer))
  (`KismetSystemLibrary.PrintString` null (`KismetTextLibrary.Conv_TextToString` (`|FormatText` "目前飞机模块得分：{score}" (`self.PlaneTotalScore`))))
  (return (`self.PlaneTotalScore`)))

(fn `RandomQuestion`
  (params (QuestionNum :type Integer))
  (locals (S_MutipleAnswerArray :type "Array of /Game/Trail/Blueprints/Questions/QuestionsData/S_MultipleAnswer Structure"))
  (`|ExecutionSequence`
    (:`then_0`
      (bind _outrownames (`DataTableFunctionLibrary.GetDataTableRowNames` "/Game/Trail/Blueprints/Questions/QuestionsData/DT_CheckPlane.DT_CheckPlane"))
      (for _array_element _outrownames
        (bind _returnvalue (`|GetDataTableRow` "/Game/Trail/Blueprints/Questions/QuestionsData/DT_CheckPlane.DT_CheckPlane" _array_element)
          (:`then`
            (`BlueprintMapLibrary.Map_Add` (`self.S_CheckPlaneMap`) (`.Index_2_F38FBE464C56B19B7AD8D89A1F7B9AE6` (break `/Game/Trail/Blueprints/Questions/QuestionsData/S_CheckPlane` _returnvalue)) _returnvalue)))))
    (:`then_1`
      (bind _outrownames_2 (`DataTableFunctionLibrary.GetDataTableRowNames` "/Game/Trail/Blueprints/Questions/QuestionsData/DT_TFImage.DT_TFImage"))
      (for _array_element_2 _outrownames_2
        (bind _returnvalue_2 (`|GetDataTableRow` "/Game/Trail/Blueprints/Questions/QuestionsData/DT_TFImage.DT_TFImage" _array_element_2)
          (:`then`
            (`BlueprintMapLibrary.Map_Add` (`self.S_TFImageMap`) (`.Index_16_B84446244B81DC1BBC1A299A7F3F741D` (break `/Game/Trail/Blueprints/Questions/QuestionsData/S_TFImage` _returnvalue_2)) _returnvalue_2)))))))