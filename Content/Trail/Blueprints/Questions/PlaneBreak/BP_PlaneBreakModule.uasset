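; BP_PlaneBreakModule is a question module that randomly picks which plane parts are broken.
; RandomQuestion extends its parent by loading all DT_PlanePart rows, shuffling them and constructing one BP_PlaneBreakQuestion per array entry.
; It flags the first QuestionNum questions as broken, though the shuffled part data is never passed to them here.
; CalculateScore is a stub that loops over the parts without computing anything.
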(fn `CalculateScore`
  (for _ (`self.S_PlanePartArray`)
    _))

(fn `RandomQuestion`
  (params (QuestionNum :type Integer))
  (`parent.RandomQuestion` QuestionNum)
  (`|ExecutionSequence`
    (:`then_0`
      (bind _outrownames (`DataTableFunctionLibrary.GetDataTableRowNames` "/Game/Trail/Blueprints/Plane/PlaneData/DT_PlanePart.DT_PlanePart"))
      (for _array_element _outrownames
        (bind _returnvalue (`|GetDataTableRow` "/Game/Trail/Blueprints/Plane/PlaneData/DT_PlanePart.DT_PlanePart" _array_element)
          (:`then`
            (`KismetArrayLibrary.Array_Add` (`self.S_PlanePartArray`) _returnvalue)))))
    (:`then_1`
      (`KismetArrayLibrary.Array_Shuffle` (`self.S_PlanePartArray`))
      (for (_ _array_index) (`self.S_PlanePartArray`)
        (bind _returnvalue_2 (`|GenericCreateObject` "/Game/Trail/Blueprints/Questions/PlaneBreak/BP_PlaneBreakQuestion.BP_PlaneBreakQuestion_C"))
        (`KismetArrayLibrary.Array_Add` (`self.PlaneBreaks`) _returnvalue_2)
        (if (< _array_index (`local.QuestionNum`))
          (set `/Game/Trail/Blueprints/Questions/PlaneBreak/BP_PlaneBreakQuestion.IsBreak` true _returnvalue_2))))))