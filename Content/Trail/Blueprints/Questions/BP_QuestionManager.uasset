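; Question manager that builds a four-level quiz and tracks the player's current level.
; GenerateQuestionnaire constructs BP_Level objects, has each generate its question modules, and passes itself as a back-reference.
; NextLevel advances a clamped index and returns that level, calling the still-empty CalculateTotalScore when the index reaches LevelNum - 1.
; PrintQuestionaire debug-prints questions by module type, including check-plane map entries, then sets CurrentLevel to Levels[LevelNum].
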(fn `AddLevelIndex`
  (bind _levelnum (`self.LevelNum`))
  (bind _returnvalue (+ (`self.CurrentLevelIndex`) 1))
  (set `self.CurrentLevelIndex` (`KismetMathLibrary.Clamp` _returnvalue 0 _levelnum))
  (if (== _returnvalue _levelnum)
    (`self.CalculateTotalScore`)))

(fn `CalculateTotalScore`)

(fn `GenerateQuestionnaire`
  (locals (Level1 :type "/Game/Trail/Blueprints/Questions/BP_Level Object Reference") (Level2 :type "/Game/Trail/Blueprints/Questions/BP_Level Object Reference") (Level3 :type "/Game/Trail/Blueprints/Questions/BP_Level Object Reference") (Level4 :type "/Game/Trail/Blueprints/Questions/BP_Level Object Reference"))
  (`|ExecutionSequence`
    (:`then_0`
      (bind _returnvalue (`|GenericCreateObject` "/Game/Trail/Blueprints/Questions/BP_Level.BP_Level_C"))
      (bind _output_get (set `local.Level1` _returnvalue))
      (`/Game/Trail/Blueprints/Questions/BP_Level.GenerateModule` _output_get 3 1 1)
      (set `/Game/Trail/Blueprints/Questions/BP_Level.QuestionManagerRef` self (`local.Level1`)))
    (:`then_1`
      (bind _returnvalue_2 (`|GenericCreateObject` "/Game/Trail/Blueprints/Questions/BP_Level.BP_Level_C"))
      (bind _output_get_2 (set `local.Level2` _returnvalue_2))
      (`/Game/Trail/Blueprints/Questions/BP_Level.GenerateModule` _output_get_2 3 1 1)
      (set `/Game/Trail/Blueprints/Questions/BP_Level.QuestionManagerRef` self (`local.Level2`)))
    (:`then_2`
      (bind _returnvalue_3 (`|GenericCreateObject` "/Game/Trail/Blueprints/Questions/BP_Level.BP_Level_C"))
      (bind _output_get_3 (set `local.Level3` _returnvalue_3))
      (`/Game/Trail/Blueprints/Questions/BP_Level.GenerateModule` _output_get_3 3 1 1)
      (set `/Game/Trail/Blueprints/Questions/BP_Level.QuestionManagerRef` self (`local.Level3`)))
    (:`then_3`
      (bind _returnvalue_4 (`|GenericCreateObject` "/Game/Trail/Blueprints/Questions/BP_Level.BP_Level_C"))
      (bind _output_get_4 (set `local.Level4` _returnvalue_4))
      (`/Game/Trail/Blueprints/Questions/BP_Level.GenerateModule` _output_get_4 3 1 1)
      (set `/Game/Trail/Blueprints/Questions/BP_Level.QuestionManagerRef` self (`local.Level4`)))
    (:`then_4`
      (set `self.Levels` (`|MakeArray` (`local.Level1`) (`local.Level2`) (`local.Level3`) (`local.Level4`)))
      (set `self.CurrentLevel` (`|GetArrayItem` (`self.Levels`))))))

(fn `Next Level`
  (returns (CurrentLevel :type "/Game/Trail/Blueprints/Questions/BP_Level Object Reference"))
  (`|ExecutionSequence`
    (:`then_0`
      (`self.AddLevelIndex`))
    (:`then_1`
      (set `self.CurrentLevel` (`|GetArrayItem` (`self.Levels`) (`self.CurrentLevelIndex`))))
    (:`then_2`
      (return (`self.CurrentLevel`)))))

(fn `PrintQuestionaire`
  (locals (QuestionModule :type "/Game/Trail/Blueprints/Questions/BP_QuestionModule Object Reference"))
  (bind _questions (`/Game/Trail/Blueprints/Questions/BP_QuestionModule.Questions` (`local.QuestionModule`)))
  (for _array_element (`self.Levels`)
    (for _array_element_2 (`/Game/Trail/Blueprints/Questions/BP_Level.BP_QuestionModuleArray` _array_element)
      (set `local.QuestionModule` _array_element_2)
      (switch `/Game/Trail/Blueprints/Questions/E_QuestionType` (`/Game/Trail/Blueprints/Questions/BP_QuestionModule.QuestionType` _array_element_2)
        (:`NewEnumerator0`
          (for _array_element_3 _questions
            (bind _asbp_single_answer_question (cast `/Game/Trail/Blueprints/Questions/SingleAnswer/BP_SingleAnswerQuestion` _array_element_3))
            (`KismetSystemLibrary.PrintString` null (`KismetTextLibrary.Conv_TextToString` (`.Question_2_88EB9CEB423053767985DFB3140F52C6` (break `/Game/Trail/Blueprints/Questions/QuestionsData/S_SingleAnswer` (`/Game/Trail/Blueprints/Questions/SingleAnswer/BP_SingleAnswerQuestion.S_SingleAnswer` _asbp_single_answer_question)))))))
        (:`NewEnumerator1`
          (for _array_element_4 _questions
            (bind _asbp_mutiple_answer_question (cast `/Game/Trail/Blueprints/Questions/MutipleAnswer/BP_MutipleAnswerQuestion` _array_element_4))
            (`KismetSystemLibrary.PrintString` null (`KismetTextLibrary.Conv_TextToString` (`.Question_2_E2B52D5C459C58C8049EB8A1705151C9` (break `/Game/Trail/Blueprints/Questions/QuestionsData/S_MultipleAnswer` (`/Game/Trail/Blueprints/Questions/MutipleAnswer/BP_MutipleAnswerQuestion.S_MutipleAnswer` _asbp_mutiple_answer_question)))))))
        (:`NewEnumerator2`
          (for _array_element_5 _questions
            (bind _asbp_trueor_false_question (cast `/Game/Trail/Blueprints/Questions/TrueorFalse/BP_TrueorFalseQuestion` _array_element_5))
            (`KismetSystemLibrary.PrintString` null (`KismetTextLibrary.Conv_TextToString` (`.Question_5_17D9ED69431B57D182F942AC0455FE04` (break `/Game/Trail/Blueprints/Questions/QuestionsData/S_TrueorFalse` (`/Game/Trail/Blueprints/Questions/TrueorFalse/BP_TrueorFalseQuestion.S_TrueorFalse` _asbp_trueor_false_question)))))))
        (:`NewEnumerator4`
          (bind _asbp_check_plane_module (cast `/Game/Trail/Blueprints/Questions/PlaneBreak/BP_CheckPlaneModule` (`local.QuestionModule`)))
          (bind _s_checkplanemap (`/Game/Trail/Blueprints/Questions/PlaneBreak/BP_CheckPlaneModule.S_CheckPlaneMap` _asbp_check_plane_module))
          (bind _keys (`BlueprintMapLibrary.Map_Keys` _s_checkplanemap))
          (for _array_element_6 _keys
            (`KismetSystemLibrary.PrintText` null (`.Question_7_353CD07841C7AC0CBEBAD6A3D37DEEAF` (break `/Game/Trail/Blueprints/Questions/QuestionsData/S_CheckPlane` (`BlueprintMapLibrary.Map_Find` _s_checkplanemap _array_element_6)))))
          (bind _s_tfimagemap (`/Game/Trail/Blueprints/Questions/PlaneBreak/BP_CheckPlaneModule.S_TFImageMap` _asbp_check_plane_module))
          (bind _keys_2 (`BlueprintMapLibrary.Map_Keys` _s_tfimagemap))
          (for _array_element_7 _keys_2
            (`KismetSystemLibrary.PrintText` null (`.Text_17_FA27A13B4E3240BF00308B8325E6AAB9` (break `/Game/Trail/Blueprints/Questions/QuestionsData/S_TFImage` (`BlueprintMapLibrary.Map_Find` _s_tfimagemap _array_element_7)))))))))
  (set `self.CurrentLevel` (`|GetArrayItem` (`self.Levels`) (`self.LevelNum`))))