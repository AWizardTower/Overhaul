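; BP_Level is the question bank for a level, holding an ordered array of question modules and tracking the current one.
; GenerateModule currently builds only a plane-check module with a random question, level reference and character transform; single-answer, multiple-answer and true/false setups are disconnected, and its count inputs are unused.
; NextModule advances the index, updates the current module and returns whether the end is reached.
; InitialPlaneModule is an empty stub for a manager.
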(fn `AddModuleIndex`
  (returns (isLevelEnd :type Boolean))
  (bind _output_get (set `self.CurrentModuleIndex` (+ (`self.CurrentModuleIndex`) 1)))
  (return (== _output_get (`KismetArrayLibrary.Array_Length` (`self.BP_QuestionModuleArray`)))))

(fn `GenerateModule`
  (params (SingleAnswerNum :type Integer) (MutipleAnswerNum :type Integer) (PlaneBrokenNum :type Integer))
  (locals (Module1 :type "/Game/Trail/Blueprints/Questions/SingleAnswer/BP_SingleAnswerModule Object Reference") (Module2 :type "/Game/Trail/Blueprints/Questions/MutipleAnswer/BP_MutipleAnswerModule Object Reference") (Module3 :type "/Game/Trail/Blueprints/Questions/TrueorFalse/BP_TrueorFalseModule Object Reference") (Module4 :type "/Game/Trail/Blueprints/Questions/PlaneBreak/BP_CheckPlaneModule Object Reference"))
  (bind _module4 (`local.Module4`))
  (`|ExecutionSequence`
    (:`then_3`
      (bind _returnvalue (`|GenericCreateObject` "/Game/Trail/Blueprints/Questions/PlaneBreak/BP_CheckPlaneModule.BP_CheckPlaneModule_C"))
      (bind _output_get (set `local.Module4` _returnvalue))
      (`/Game/Trail/Blueprints/Questions/BP_QuestionModule.RandomQuestion` _output_get 0)
      (set `/Game/Trail/Blueprints/Questions/BP_QuestionModule.LevelRef` self _module4)
      (set `/Game/Trail/Blueprints/Questions/BP_QuestionModule.CharacterLocation` (`KismetMathLibrary.MakeTransform` (20195.0 -11344.0 200.0) (struct :`Yaw` 176.0)) _module4))
    (:`then_4`
      (bind _output_get_2 (set `self.BP_QuestionModuleArray` (`|MakeArray` (`local.Module4`) null null null :!type "/Game/Trail/Blueprints/Questions/BP_QuestionModule Object Reference")))
      (set `self.CurrentQuestionModule` (`|GetArrayItem` _output_get_2)))))

(fn `InitialPlaneModule`)

(fn `NextModule`
  (returns (isLevelEnd :type Boolean))
  (`KismetSystemLibrary.PrintString` null "题库中切换到下一题型")
  (`|ExecutionSequence`
    (:`then_0`
      (bind _islevelend (`self.AddModuleIndex`)))
    (:`then_1`
      (set `self.CurrentQuestionModule` (`|GetArrayItem` (`self.BP_QuestionModuleArray`) (`self.CurrentModuleIndex`)))
      (return _islevelend))))