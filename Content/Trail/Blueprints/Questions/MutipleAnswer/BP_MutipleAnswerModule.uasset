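; Multiple-answer question module that loads quiz questions from the DT_MultipleAnswer data table.
; RandomQuestion walks every row, caches found row structs and wraps each row in a new BP_MutipleAnswerQuestion object added to the Questions list.
; CurrentQuestion is set to the first entry in that list.
; Despite the function name, no shuffling occurs and the QuestionNum input is unused.
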(fn `RandomQuestion`
  (params (QuestionNum :type Integer))
  (bind _outrownames (`DataTableFunctionLibrary.GetDataTableRowNames` "/Game/Trail/Blueprints/Questions/QuestionsData/DT_MultipleAnswer.DT_MultipleAnswer"))
  (for _array_element _outrownames
    (`|ExecutionSequence`
      (:`then_0`
        (bind _returnvalue (`|GetDataTableRow` "/Game/Trail/Blueprints/Questions/QuestionsData/DT_MultipleAnswer.DT_MultipleAnswer" _array_element)
          (:`then`
            (`KismetArrayLibrary.Array_Add` (`self.S_MutipleAnswerArray`) _returnvalue))))
      (:`then_1`
        (bind _returnvalue_2 (`|GenericCreateObject` "/Game/Trail/Blueprints/Questions/MutipleAnswer/BP_MutipleAnswerQuestion.BP_MutipleAnswerQuestion_C"))
        (set `/Game/Trail/Blueprints/Questions/MutipleAnswer/BP_MutipleAnswerQuestion.S_MutipleAnswer` _returnvalue _returnvalue_2)
        (`KismetArrayLibrary.Array_Add` (`self.Questions`) _returnvalue_2))
      (:`then_2`
        (set `self.CurrentQuestion` (`|GetArrayItem` (`self.Questions`)))))))