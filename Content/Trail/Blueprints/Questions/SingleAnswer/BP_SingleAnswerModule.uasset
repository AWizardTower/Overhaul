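; Single-answer question module that builds its question pool from the DT_SingleAnswer data table.
; RandomQuestion loops over every row, caching its data in SingleAnswerQuestions and wrapping it in a new BP_SingleAnswerQuestion object added to Questions.
; CurrentQuestion is always set to the first entry; despite the function name, nothing is randomized and QuestionNum is unused.
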(fn `RandomQuestion`
  (params (QuestionNum :type Integer))
  (bind _outrownames (`DataTableFunctionLibrary.GetDataTableRowNames` "/Game/Trail/Blueprints/Questions/QuestionsData/DT_SingleAnswer.DT_SingleAnswer"))
  (for _array_element _outrownames
    (`|ExecutionSequence`
      (:`then_0`
        (bind _returnvalue (`|GetDataTableRow` "/Game/Trail/Blueprints/Questions/QuestionsData/DT_SingleAnswer.DT_SingleAnswer" _array_element)
          (:`then`
            (`KismetArrayLibrary.Array_Add` (`self.SingleAnswerQuestions`) _returnvalue))))
      (:`then_1`
        (bind _returnvalue_2 (`|GenericCreateObject` "/Game/Trail/Blueprints/Questions/SingleAnswer/BP_SingleAnswerQuestion.BP_SingleAnswerQuestion_C"))
        (bind _output_get (set `/Game/Trail/Blueprints/Questions/SingleAnswer/BP_SingleAnswerQuestion.S_SingleAnswer` _returnvalue _returnvalue_2))
        (`KismetArrayLibrary.Array_Add` (`self.Questions`) _returnvalue_2))
      (:`then_2`
        (set `self.CurrentQuestion` (`|GetArrayItem` (`self.Questions`)))))))